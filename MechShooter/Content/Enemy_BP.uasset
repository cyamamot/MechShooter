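; Enemy actor Blueprint that takes point and radial damage and shows its health on a floating widget.
; Each tick it turns the widget toward the player camera and copies current and max health into the Enemy_UI user widget.
; Both damage events print and subtract the amount, then at zero health share a branch that spawns a scaled-up explosion emitter and destroys the actor.
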(event `self.ReceiveTick`
  (params (DeltaSeconds :type "Float (single-precision)"))
  (bind _widget (`self.Widget`))
  (`SceneComponent.K2_SetWorldRotation` _widget (`KismetMathLibrary.FindLookAtRotation` (`SceneComponent.K2_GetComponentLocation` _widget) (`PlayerCameraManager.GetCameraLocation` (`GameplayStatics.GetPlayerCameraManager` 0))) false false)
  (bind _asenemy_ui (cast `/Game/Enemy_UI` (`WidgetComponent.GetUserWidgetObject` (`self.Widget`))))
  (set `/Game/Enemy_UI.EnemyHealth` (`self.Health`) _asenemy_ui)
  (set `/Game/Enemy_UI.EnemyMaxHealth` (`self.MaxHealth`) _asenemy_ui))

(event `self.ReceivePointDamage`
  (params (Damage :type "Float (single-precision)") (DamageType :type "DamageType Object Reference") (HitLocation :type "Vector Structure") (HitNormal :type "Vector Structure") (HitComponent :type "PrimitiveComponent Object Reference") (BoneName :type Name) (ShotFromDirection :type "Vector Structure") (InstigatedBy :type "Controller Object Reference") (DamageCauser :type "Actor Object Reference") (HitInfo :type "HitResult Structure (by ref)"))
  (`KismetSystemLibrary.PrintString` (`KismetStringLibrary.Conv_DoubleToString` Damage))
  (bind _output_get (set `self.Health` (- (`self.Health`) Damage)))
  (if (<= _output_get 0.0)
    (bind _returnvalue (`GameplayStatics.SpawnEmitterAtLocation` "/Game/FX/Particles/P_Explosion.P_Explosion" (`self.K2_GetActorLocation` self) :!label _label))
    (`SceneComponent.SetRelativeScale3D` _returnvalue (5.0 5.0 5.0))
    (`self.K2_DestroyActor`)))

(event `self.ReceiveRadialDamage`
  (params (DamageReceived :type "Float (single-precision)") (DamageType :type "DamageType Object Reference") (Origin :type "Vector Structure") (HitInfo :type "HitResult Structure (by ref)") (InstigatedBy :type "Controller Object Reference") (DamageCauser :type "Actor Object Reference"))
  (`KismetSystemLibrary.PrintString` (`KismetStringLibrary.Conv_DoubleToString` DamageReceived))
  (bind _output_get (set `self.Health` (- (`self.Health`) DamageReceived)))
  (if (<= _output_get 0.0)
    (goto _label)))

(fn `UserConstructionScript`)