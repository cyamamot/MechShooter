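; MechCharacter_BP is a mech player character Blueprint with first-person and third-person cameras.
; Each tick it sets the first-person camera's relative pitch from the control rotation, with roll and yaw held at zero.
; A SwitchCamera event toggles both cameras' active states, and a QuitGame input action quits the game.
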(event `self.ReceiveTick`
  (params (DeltaSeconds :type "Float (single-precision)"))
  (bind (_returnvalue_roll _returnvalue_pitch) (`KismetMathLibrary.BreakRotator` (`self.GetControlRotation`)))
  (`SceneComponent.K2_SetRelativeRotation` (`self.FPCamera`) (`KismetMathLibrary.MakeRotator` 0.0 _returnvalue_pitch) false false))

(event `SwitchCamera`
  (`ActorComponent.ToggleActive` (`self.TPCamera`))
  (`ActorComponent.ToggleActive` (`self.FPCamera`)))

(event `InputAction|QuitGame`
  (params (Key :type "Key Structure" :default "AnyKey"))
  (:`Pressed`
    (`KismetSystemLibrary.QuitGame` (`GameplayStatics.GetPlayerController` 0) "Quit")))

(fn `UserConstructionScript`)