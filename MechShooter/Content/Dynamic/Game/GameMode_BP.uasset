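; Game mode that opens the game on a start menu and handles the win condition of clearing all enemies.
; On BeginPlay it pauses the game, disables pawn input and shows StartMenu_BP in UI-only input mode.
; CheckEnemies recounts living Enemy_BP actors on each call and triggers Win when none remain.
; Win displays MissionEnd_BP and calls MoveUp on the first Door_BP found in the level.
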(event `self.ReceiveBeginPlay`
  (bind _returnvalue (`GameplayStatics.GetPlayerController` 0))
  (`GameplayStatics.SetGamePaused` true)
  (`self.DisableInput` (`GameplayStatics.GetPlayerPawn` 0) _returnvalue)
  (set `PlayerController.bShowMouseCursor` true _returnvalue)
  (bind _returnvalue_2 (`|CreateWidget` "/Game/Dynamic/Game/StartMenu_BP.StartMenu_BP_C"))
  (`UserWidget.AddToViewport` _returnvalue_2 0)
  (`WidgetBlueprintLibrary.SetInputMode_UIOnlyEx` (`GameplayStatics.GetPlayerController` 0) _returnvalue_2 "LockAlways"))

(event `CheckEnemies`
  (set `self.NumberOfEnemiesAlive` 0)
  (bind _outactors (`GameplayStatics.GetAllActorsOfClass` "/Game/Dynamic/Enemy/Enemy_BP.Enemy_BP_C"))
  (bind _output_get (set `self.CurrentEnemies` _outactors))
  (for _array_element _output_get
    (bind _asenemy_bp (cast `/Game/Dynamic/Enemy/Enemy_BP` _array_element))
    (if (`/Game/Dynamic/Enemy/Enemy_BP.IsAlive` _asenemy_bp)
      (set `self.NumberOfEnemiesAlive` (+ (`self.NumberOfEnemiesAlive`) 1))))
  (if (== (`self.NumberOfEnemiesAlive`) 0)
    (`self.Win`)))

(event `Win`
  (bind _returnvalue (`|CreateWidget` "/Game/Dynamic/Game/MissionEnd_BP.MissionEnd_BP_C"))
  (`UserWidget.AddToViewport` _returnvalue 0)
  (bind _outactors (`GameplayStatics.GetAllActorsOfClass` "/Game/Static/Game/MapObjects/Pillars/Door_BP.Door_BP_C"))
  (`/Game/Static/Game/MapObjects/Pillars/Door_BP.MoveUp` (`|GetArrayItem` _outactors)))

(fn `UserConstructionScript`)