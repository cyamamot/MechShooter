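; Enemy Blueprint for a bobbing enemy that takes point and radial damage and shows a health widget.
; Tick turns the widget toward the camera, feeds it health and scales it by distance to the player.
; Damage or MechCharacter_BP proximity reveals the widget, with delayed hiding.
; At zero health a one-shot Death stops the bob, drops the mesh with physics, then spawns smoke and sparks, leaving the actor in place.
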(event `self.ReceiveBeginPlay`
  (bind (_direction _bobble) (`Timeline|EnemyBob` :!label _label)
    (:`Update`
      (`SceneComponent.K2_AddLocalOffset` (`self.StaticMesh`) (`KismetMathLibrary.MakeVector` 0.0 0.0 (* _bobble 5.0)) false false))))

(event `StopBob`
  (goto _label :!via `Stop`))

(event `Death`
  (bind _staticmesh (`self.StaticMesh`))
  (bind _returnvalue (`SceneComponent.K2_GetComponentLocation` _staticmesh))
  (`/Engine/EditorBlueprintResources/StandardMacros.DoOnce` false
    (:`Completed`
      (`PrimitiveComponent.SetCollisionEnabled` (`self.Box`) "NoCollision")
      (set `self.IsAlive` false)
      (`SceneComponent.SetVisibility` (`self.Widget`) false false)
      (`self.StopBob`)
      (`PrimitiveComponent.SetSimulatePhysics` _staticmesh true)
      (`PrimitiveComponent.SetEnableGravity` _staticmesh true)
      (`KismetSystemLibrary.Delay` 1.0)
      (`PrimitiveComponent.SetSimulatePhysics` _staticmesh false)
      (bind _returnvalue_2 (`GameplayStatics.SpawnEmitterAtLocation` "/Game/Dynamic/FX/Particles/P_Smoke.P_Smoke" _returnvalue (struct) false))
      (`SceneComponent.SetRelativeScale3D` _returnvalue_2 (3.0 3.0 7.0))
      (bind _returnvalue_3 (`GameplayStatics.SpawnEmitterAtLocation` "/Game/Dynamic/FX/Particles/P_Sparks.P_Sparks" _returnvalue (struct) false))
      (`SceneComponent.SetRelativeScale3D` _returnvalue_3 (3.0 3.0 3.0)))))

(event `self.ReceiveTick`
  (params (DeltaSeconds :type "Float (single-precision)"))
  (bind _widget (`self.Widget`))
  (bind _returnvalue (`WidgetComponent.GetUserWidgetObject` (`self.Widget`)))
  (bind _returnvalue_2 (/ (`KismetMathLibrary.FClamp` (`KismetMathLibrary.VSize` (- (`SceneComponent.K2_GetComponentLocation` (`self.StaticMesh`)) (`self.K2_GetActorLocation` (`GameplayStatics.GetPlayerPawn` 0)))) 750.0 2000.0) 750.0))
  (`SceneComponent.K2_SetWorldRotation` _widget (`KismetMathLibrary.FindLookAtRotation` (`SceneComponent.K2_GetComponentLocation` _widget) (`PlayerCameraManager.GetCameraLocation` (`GameplayStatics.GetPlayerCameraManager` 0))) false false)
  (bind _asenemy_ui (cast `/Game/Dynamic/Enemy/Enemy_UI` _returnvalue))
  (set `/Game/Dynamic/Enemy/Enemy_UI.EnemyHealth` (`self.Health`) _asenemy_ui)
  (set `/Game/Dynamic/Enemy/Enemy_UI.EnemyMaxHealth` (`self.MaxHealth`) _asenemy_ui)
  (`Widget.SetRenderScale` _returnvalue (`KismetMathLibrary.MakeVector2D` _returnvalue_2 _returnvalue_2)))

(event `self.ReceivePointDamage`
  (params (Damage :type "Float (single-precision)") (DamageType :type "DamageType Object Reference") (HitLocation :type "Vector Structure") (HitNormal :type "Vector Structure") (HitComponent :type "PrimitiveComponent Object Reference") (BoneName :type Name) (ShotFromDirection :type "Vector Structure") (InstigatedBy :type "Controller Object Reference") (DamageCauser :type "Actor Object Reference") (HitInfo :type "HitResult Structure (by ref)"))
  (bind _widget (`self.Widget`))
  (if (`self.IsAlive`)
    (set `self.DamageCauser` DamageCauser)
    (`SceneComponent.SetVisibility` _widget true false)
    (bind _asenemy_ui (cast `/Game/Dynamic/Enemy/Enemy_UI` (`WidgetComponent.GetUserWidgetObject` _widget)))
    (set `/Game/Dynamic/Enemy/Enemy_UI.VisibileState` "Hidden" _asenemy_ui)
    (bind _output_get (set `/Game/Dynamic/Enemy/Enemy_UI.DamageDealt` Damage _asenemy_ui))
    (set `/Game/Dynamic/Enemy/Enemy_UI.VisibileState` "Visible" _asenemy_ui)
    (bind _output_get_2 (set `self.Health` (- (`self.Health`) _output_get)))
    (if (<= _output_get_2 0.0)
      (`self.Death` :!label _label_2)
      (else
        (`/Engine/EditorBlueprintResources/StandardMacros.IsValid` _asenemy_ui
          (:`Is Valid`
            (`/Game/Dynamic/Enemy/Enemy_UI.DamageAnim` _asenemy_ui)
            (`KismetSystemLibrary.Delay` 0.5)
            (set `/Game/Dynamic/Enemy/Enemy_UI.VisibileState` "Hidden" _asenemy_ui)
            (`KismetSystemLibrary.RetriggerableDelay` 6.0)
            (`SceneComponent.SetVisibility` (`self.Widget`) false false)))))))

(event `self.ReceiveRadialDamage`
  (params (DamageReceived :type "Float (single-precision)") (DamageType :type "DamageType Object Reference") (Origin :type "Vector Structure") (HitInfo :type "HitResult Structure (by ref)") (InstigatedBy :type "Controller Object Reference") (DamageCauser :type "Actor Object Reference"))
  (bind _widget (`self.Widget`))
  (if (`self.IsAlive`)
    (set `self.DamageCauser` DamageCauser)
    (`SceneComponent.SetVisibility` _widget true false)
    (bind _asenemy_ui (cast `/Game/Dynamic/Enemy/Enemy_UI` (`WidgetComponent.GetUserWidgetObject` _widget)))
    (set `/Game/Dynamic/Enemy/Enemy_UI.VisibileState` "Hidden" _asenemy_ui)
    (bind _output_get (set `/Game/Dynamic/Enemy/Enemy_UI.DamageDealt` DamageReceived _asenemy_ui))
    (set `/Game/Dynamic/Enemy/Enemy_UI.VisibileState` "Visible" _asenemy_ui)
    (bind _output_get_2 (set `self.Health` (- (`self.Health`) _output_get)))
    (if (<= _output_get_2 0.0)
      (goto _label_2)
      (else
        (`/Engine/EditorBlueprintResources/StandardMacros.IsValid` _asenemy_ui
          (:`Is Valid`
            (`/Game/Dynamic/Enemy/Enemy_UI.DamageAnim` _asenemy_ui)
            (`KismetSystemLibrary.Delay` 0.5)
            (set `/Game/Dynamic/Enemy/Enemy_UI.VisibileState` "Hidden" _asenemy_ui)
            (`KismetSystemLibrary.RetriggerableDelay` 6.0)
            (`SceneComponent.SetVisibility` (`self.Widget`) false false)))))))

(event `self.NotificationBox.OnComponentBeginOverlap`
  (params (OverlappedComponent :type "PrimitiveComponent Object Reference") (OtherActor :type "Actor Object Reference") (OtherComp :type "PrimitiveComponent Object Reference") (OtherBodyIndex :type Integer) (bFromSweep :type Boolean) (SweepResult :type "HitResult Structure (by ref)"))
  (cast `/Game/Dynamic/MechCharacter/MechCharacter_BP` OtherActor)
  (if (`self.IsAlive`)
    (`SceneComponent.SetVisibility` (`self.Widget`) true false)))

(event `self.NotificationBox.OnComponentEndOverlap`
  (params (OverlappedComponent :type "PrimitiveComponent Object Reference") (OtherActor :type "Actor Object Reference") (OtherComp :type "PrimitiveComponent Object Reference") (OtherBodyIndex :type Integer))
  (cast `/Game/Dynamic/MechCharacter/MechCharacter_BP` OtherActor)
  (if (`self.IsAlive`)
    (`KismetSystemLibrary.Delay` 3.0)
    (`SceneComponent.SetVisibility` (`self.Widget`) false false)))

(fn `UserConstructionScript`)